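; BP_GirlController is a controller Blueprint that keeps the two player characters' meshes mirrored relative to each other.
; On BeginPlay it prints its platform user ID.
; Every Tick it resets player 0's mesh to normal world scale and flips player 1's mesh with a negative Y scale.
; The branch condition is fixed to true, so the reversed assignment never runs.
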(event EventBeginPlay
  (Development|PrintString (Utilities|String|ToString(Integer) (Class|PlayerController|GetPlatformUserId))))

(event EventTick
  (params (DeltaSeconds :type Float%20%28single-precision%29))
  (if true
    (Transformation|SetWorldScale3D (Variables|/Script/Engine.Character|GetMesh (Game|GetPlayerCharacter 0)) "1.000000,1.000000,1.000000")
    (Transformation|SetWorldScale3D (Variables|/Script/Engine.Character|GetMesh (Game|GetPlayerCharacter 1)) "1.000000,-1.000000,1.000000")
    (else
      (Transformation|SetWorldScale3D (Variables|/Script/Engine.Character|GetMesh (Game|GetPlayerCharacter 0)) "1.000000,-1.000000,1.000000")
      (Transformation|SetWorldScale3D (Variables|/Script/Engine.Character|GetMesh (Game|GetPlayerCharacter 1)) "1.000000,1.000000,1.000000"))))

(fn ConstructionScript)