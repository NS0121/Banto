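; Girl player character Blueprint that registers its Enhanced Input mapping on BeginPlay and turns lever input into side-to-side movement along the world Y axis.
; The lever vector becomes an angle, which Allocation sorts into eight numpad-style direction codes.
; Only left (4) and right (6) drive movement so far.
; Beacon, jump, gauge special and punch inputs are placeholders that print debug strings.
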(event Input|EnhancedActionEvents|EnhancedInputActionIA_Lever
  (params (ActionValue :type Vector%202D%20Structure) (ElapsedSeconds :type Float%20%28double-precision%29) (TriggeredSeconds :type Float%20%28double-precision%29) (InputAction :type Input%20Action%20Object%20Reference :default "/Game/Member/Namiki/BP/Char/Input/Action/IA_Lever.IA_Lever"))
  (:Triggered
    (bind _returnvalue (Class|CPPCharBase|FromPointtoPointtoAngle (.x ActionValue) (.y ActionValue)))
    (bind _num (CallFunction|Allocation _returnvalue))
    (switch int _num
      (:4
        ;[1 1 1] 4
        (bind _output_get (Variables|/Script/Engine.CharacterMovementComponent|SetMaxWalkSpeed (Variables|Character|GetCharacterMovement) 6e+02))
        (Pawn|Input|AddMovementInput "0.000000,1.000000,0.000000" (* _output_get -1.0) false))
      (:6
        ;[1 1 1] 6
        (Variables|/Script/Engine.CharacterMovementComponent|SetMaxWalkSpeed (Variables|Character|GetCharacterMovement) 6e+02)
        (Pawn|Input|AddMovementInput "0.000000,1.000000,0.000000" 1.0 false)))))

(event Input|EnhancedActionEvents|EnhancedInputActionIA_Beacon
  (params (ActionValue :type Boolean) (ElapsedSeconds :type Float%20%28double-precision%29) (TriggeredSeconds :type Float%20%28double-precision%29) (InputAction :type Input%20Action%20Object%20Reference :default "/Game/Member/Namiki/BP/Char/Input/Action/IA_Beacon.IA_Beacon"))
  ;[1 1 1] ビーコン
  (:Started
    (Development|PrintString "Flag")))

(event Input|EnhancedActionEvents|EnhancedInputActionIA_Jumpp
  (params (ActionValue :type Boolean) (ElapsedSeconds :type Float%20%28double-precision%29) (TriggeredSeconds :type Float%20%28double-precision%29) (InputAction :type Input%20Action%20Object%20Reference :default "/Game/Member/Namiki/BP/Char/Input/Action/IA_Jumpp.IA_Jumpp"))
  ;[1 1 1] ジャンプ
  (:Started
    (Development|PrintString "jump")))

(event Input|EnhancedActionEvents|EnhancedInputActionIA_Special
  (params (ActionValue :type Boolean) (ElapsedSeconds :type Float%20%28double-precision%29) (TriggeredSeconds :type Float%20%28double-precision%29) (InputAction :type Input%20Action%20Object%20Reference :default "/Game/Member/Namiki/BP/Char/Input/Action/IA_Special.IA_Special"))
  ;[1 1 1] ゲージ技
  (:Started
    (Development|PrintString "Special")))

(event Input|EnhancedActionEvents|EnhancedInputActionIA_Punch
  (params (ActionValue :type Boolean) (ElapsedSeconds :type Float%20%28double-precision%29) (TriggeredSeconds :type Float%20%28double-precision%29) (InputAction :type Input%20Action%20Object%20Reference :default "/Game/Member/Namiki/BP/Char/Input/Action/IA_Punch.IA_Punch"))
  ;[1 1 1] 攻撃
  (:Started
    (Development|PrintString "Punch")))

(event EventBeginPlay
  (bind _asplayer_controller (Utilities|Casting|CastToPlayerController (Pawn|GetController)))
  (Utilities|IsValid (PlayerController|LocalPlayerSubsystems|GetEnhancedInputLocalPlayerSubsystem _asplayer_controller)
    (:Is%20Valid
      (Input|AddMappingContext (PlayerController|LocalPlayerSubsystems|GetEnhancedInputLocalPlayerSubsystem _asplayer_controller) "/Game/Member/Namiki/BP/Char/Input/IMC_Girl.IMC_Girl" 0 "(bIgnoreAllPressedKeysUntilRelease=True,bForceImmediately=False)"))))

(event EventTick
  (params (DeltaSeconds :type Float%20%28single-precision%29)))

(fn ConstructionScript)

(fn Allocation
  (params (Angle :type Float%20%28double-precision%29))
  (if (Math|Float|InRange(Float) Angle 2.1e+02 2.4e+02)
    (return 1)
    (elif (Math|Float|InRange(Float) Angle 2.4e+02 3e+02)
      (return 2)
      (elif (Math|Float|InRange(Float) Angle 3e+02 3.3e+02)
        (return 3)
        (elif (Math|Float|InRange(Float) Angle 1.5e+02 2.1e+02)
          (return 4)
          (elif (or (> Angle 3.3e+02) (< Angle 3e+01))
            (return 6)
            (elif (Math|Float|InRange(Float) Angle 1.2e+02 1.5e+02)
              (return 7)
              (elif (Math|Float|InRange(Float) Angle 6e+01 1.2e+02)
                (return 8)
                (elif (Math|Float|InRange(Float) Angle 3e+01 6e+01)
                  (return 9))))))))))