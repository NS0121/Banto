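; Player 1 character Blueprint for a versus game against BPC_Girl02, with punches and a knife-carrying objective.
; Hits from Girl02's punch trigger brief global slow-motion hit stop, disabled input and physics knockback away from the enemy.
; PunchEvent toggles the punch collision.
; IA_Knife shows the knife in one Y zone, then in the opposite zone hides it and spawns a randomly placed actor via a re-armed DoOnce, calling the 1P win at five.
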(event OnComponentBeginOverlap(CapsuleComponent)
  (params (OverlappedComponent :type Primitive%20Component%20Object%20Reference) (OtherActor :type Actor%20Object%20Reference) (OtherComp :type Primitive%20Component%20Object%20Reference) (OtherBodyIndex :type Integer) (bFromSweep :type Boolean) (SweepResult :type Hit%20Result%20Structure%20%28by%20ref%29))
  (bind _returnvalue (Components|ComponentHasTag OtherComp "Girl02Punch"))
  ;[1 1 1] 被弾時
  (if _returnvalue
    (Variables|Default|SetIsHitDamage _returnvalue)
    ;[1 1 1] ヒットストップ
    (Utilities|Time|SetGlobalTimeDilation 0.1)
    (Utilities|FlowControl|Delay (stale EventTick DeltaSeconds))
    (Utilities|Time|SetGlobalTimeDilation 1.0)
    ;[1 1 1] 入力拒否
    (Input|DisableInput (Game|GetPlayerController 0))
    ;[1 1 1] ノックバック
    (if (> (.y (Transformation|GetActorLocation)) (.y (Transformation|GetActorLocation (Variables|Default|GetEnemy))))
      (Physics|SetSimulatePhysics (Variables|Default|GetCapsuleComponent) true)
      (Physics|AddForce (Variables|Default|GetCapsuleComponent) "0.000000,4000000.000000,0.000000" "None" false)
      (else
        (Physics|SetSimulatePhysics (Variables|Default|GetCapsuleComponent) true)
        (Physics|AddForce (Variables|Default|GetCapsuleComponent) "0.000000,-4000000.000000,0.000000" "None" false)))
    (Utilities|FlowControl|Delay 1.0)
    ;[1 1 1] 解除
    (Input|EnableInput (Game|GetPlayerController 0))
    (Physics|SetSimulatePhysics (Variables|Default|GetCapsuleComponent) false)
    (Variables|Default|SetIsHitDamage false)))

(event Input|EnhancedActionEvents|EnhancedInputActionIA_Knife
  (params (ActionValue :type Boolean) (ElapsedSeconds :type Float%20%28double-precision%29) (TriggeredSeconds :type Float%20%28double-precision%29) (InputAction :type Input%20Action%20Object%20Reference :default "/Game/Member/Namiki/BP/Char/Input/Action/IA_Knife.IA_Knife"))
  (bind _returnvalue (Math|Random|RandomFloatinRange -2e+01 2e+01))
  (bind _returnvalue_2 (Transformation|GetActorLocation))
  ;[1 1 1] ナイフ
  (:Started
    (Utilities|FlowControl|Sequence
      (:then_0
        (if (Math|Float|InRange(Float) (.y _returnvalue_2) -6.1e+02 -5.1e+02)
          (Rendering|SetVisibility (Variables|Default|GetKnife) true false)
          (goto _label Reset)))
      (:then_1
        (if (Math|Float|InRange(Float) (.y _returnvalue_2) 5.1e+02 6.1e+02)
          (Utilities|FlowControl|DoOnce true :!label _label
            (:Completed
              (Rendering|SetVisibility (Variables|Default|GetKnife) false false)
              (Game|SpawnActorfromClass "/Game/Member/Namiki/BP/BP_Knife.BP_Knife_C" (Math|Transform|MakeTransform (Math|Vector|MakeVector 955.0 (Math|Random|RandomFloatinRange 525.0 575.0) (Math|Random|RandomFloatinRange -1e+01 55.0)) (Math|Rotator|MakeRotator _returnvalue 0.0 (+ _returnvalue 9e+01)) "1.000000,1.000000,1.000000") "Undefined" 0 0)
              (Variables|Default|SetKnifeCount (+ (Variables|Default|GetKnifeCount) 1))
              (if (>= (Variables|Default|GetKnifeCount) 5)
                (Default|CallKnifeWin1P)))))))))

(event EventBeginPlay
  (|CallParentFunction)
  (bind _outactors (Actor|GetAllActorsOfClass "/Game/Member/Namiki/BP/Char/Girl02/BPC_Girl02.BPC_Girl02_C"))
  (for _array_element _outactors
    (Variables|Default|SetEnemy _array_element)))

(event Collision|EventActorBeginOverlap
  (params (OtherActor :type Actor%20Object%20Reference))
  (|CallParentFunction OtherActor) ; このノードは無効になっているため呼び出せません。\n機能をビルドするにはピンをドラッグしてください。
)

(event EventTick
  (params (DeltaSeconds :type Float%20%28single-precision%29))
  (|CallParentFunction DeltaSeconds))

(event EventPunchEvent
  (params (IsOverlap :type Boolean))
  ;[1 1 1] パンチ攻撃時の判定
  (if IsOverlap
    (Collision|SetCollisionEnabled (Variables|Default|GetPunch) "QueryAndPhysics")
    (else
      (Collision|SetCollisionEnabled (Variables|Default|GetPunch) "NoCollision"))))

(fn ConstructionScript
  (|CallParentFunction))