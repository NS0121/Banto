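; Breakable fence actor that crumbles in stages when player characters hit it.
; Overlaps on the Break component count only for Player-tagged BPC_Girl01 or BPC_Girl02 actors with IsHitDamage set.
; Each counted hit swaps to the next fence mesh until the last is hidden and the actor is destroyed.
; A DoOnce precedes these checks and resets only after a delayed stage swap, so a non-qualifying overlap leaves it closed.
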(event OnComponentBeginOverlap(Break)
  (params (OverlappedComponent :type Primitive%20Component%20Object%20Reference) (OtherActor :type Actor%20Object%20Reference) (OtherComp :type Primitive%20Component%20Object%20Reference) (OtherBodyIndex :type Integer) (bFromSweep :type Boolean) (SweepResult :type Hit%20Result%20Structure%20%28by%20ref%29))
  (Utilities|FlowControl|DoOnce false :!label _label
    (:Completed
      (if (Actor|ActorHasTag OtherActor "Player")
        (Utilities|FlowControl|Sequence
          (:then_0
            (bind _asbpc_girl_01 (Utilities|Casting|CastToBPC_Girl01 OtherActor))
            (if (Variables|/Game/Member/Namiki/BP/Char/BPC_Base.BPC_Base_C|GetIsHitDamage _asbpc_girl_01)
              ;[1 1 1] フェンスを徐々に破壊
              (Variables|Default|SetBreakCount (+ (Variables|Default|GetBreakCount) 1) :!label _label_2)
              (switch int (Variables|Default|GetBreakCount)
                (:1
                  (Rendering|SetVisibility (Variables|Default|GetFenc01) false false)
                  (Rendering|SetVisibility (Variables|Default|GetFenc02) true false)
                  (Utilities|FlowControl|Delay 1.0 :!label _label_3)
                  (goto _label Reset))
                (:2
                  (Rendering|SetVisibility (Variables|Default|GetFenc02) false false)
                  (Rendering|SetVisibility (Variables|Default|GetFenc03) true false)
                  (goto _label_3))
                (:3
                  (Rendering|SetVisibility (Variables|Default|GetFenc03) false false)
                  (Rendering|SetVisibility (Variables|Default|GetFenc04) true false)
                  (goto _label_3))
                (:4
                  (Rendering|SetVisibility (Variables|Default|GetFenc04) false false)
                  (Utilities|FlowControl|Delay 0.2)
                  (Actor|DestroyActor)))))
          (:then_1
            (bind _asbpc_girl_02 (Utilities|Casting|CastToBPC_Girl02 OtherActor))
            (if (Variables|/Game/Member/Namiki/BP/Char/BPC_Base.BPC_Base_C|GetIsHitDamage _asbpc_girl_02)
              (goto _label_2))))))))

(event EventBeginPlay
  (Rendering|SetVisibility (Variables|Default|GetFenc02) false false)
  (Rendering|SetVisibility (Variables|Default|GetFenc03) false false)
  (Rendering|SetVisibility (Variables|Default|GetFenc04) false false))

(event Collision|EventActorBeginOverlap
  (params (OtherActor :type Actor%20Object%20Reference)))

(event EventTick
  (params (DeltaSeconds :type Float%20%28single-precision%29)))

(fn ConstructionScript)